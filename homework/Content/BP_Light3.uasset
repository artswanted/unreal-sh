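; BP_Light3 is a spotlight Blueprint that switches its light on and off for a short fixed sequence when play begins.
; The construction script sets the SpotLight's starting visibility from the IsEnable variable.
; BeginPlay runs an unrolled chain of four evenly spaced delays and visibility toggles without looping, so the light ends in the state it started in.
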(event `self.ReceiveBeginPlay`
  (bind _spotlight (`self.SpotLight`))
  (`KismetSystemLibrary.Delay` 2.0)
  (`SceneComponent.ToggleVisibility` _spotlight false)
  (`KismetSystemLibrary.Delay` 2.0)
  (`SceneComponent.ToggleVisibility` _spotlight false)
  (`KismetSystemLibrary.Delay` 2.0)
  (`SceneComponent.ToggleVisibility` _spotlight false)
  (`KismetSystemLibrary.Delay` 2.0)
  (`SceneComponent.ToggleVisibility` _spotlight false))

(fn `UserConstructionScript`
  (`SceneComponent.SetVisibility` (`self.SpotLight`) (`self.isEnable`) false))